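; BeatNight game mode that runs short and long rhythm timers and rebuilds the player's saved weapon inventory.
; Tick starts two self-restarting Delay loops once, which pulse ShortActVar and LongActVar on a beat.
; SetLoadInventorytoPlayer copies weapon arrays from the load game instance, then spawns swords, guns and rope by type and name.
; Per-weapon graphs restore level or ammo, attach each weapon to its saved BP_Inventory slot, and fill Player.Inventory.
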(event EventTick
  (params (DeltaSeconds :type Float%20%28single-precision%29))
  ;[1 1 1] 짧은 리듬
  (Utilities|FlowControl|Sequence
    (:then_0
      (if (not (Variables|Default|Getwhat))
        (Utilities|FlowControl|Sequence
          (:then_0
            (bind _output_get (Variables|Default|SetShortActCool 0.0 :!label _label))
            (if (< _output_get 1.0)
              (Variables|Default|SetShortActVar false)
              (Utilities|FlowControl|Delay 0.5 :!label _label_2)
              (bind _output_get_2 (Variables|Default|SetShortActCool (+ (Variables|Default|GetShortActCool) 1.0)))
              (if (== _output_get_2 1.0)
                (Variables|Default|SetShortActVar true)
                (Utilities|FlowControl|Delay 0.2)
                (goto _label)
                (else
                  (goto _label_2)))))
          (:then_1
            (Variables|Default|Setwhat true)))))
    (:then_1
      ;[1 1 1] 긴 리듬
      (if (not (Variables|Default|Getwhat2))
        (Utilities|FlowControl|Sequence
          (:then_0
            (bind _output_get_3 (Variables|Default|SetLongActCool 0.0 :!label _label_3))
            (if (< _output_get_3 1.0)
              (Variables|Default|SetLongActVar false)
              (Utilities|FlowControl|Delay 0.5)
              (Variables|Default|SetLongActCool (+ (Variables|Default|GetLongActCool) 0.5))
              (Utilities|FlowControl|Delay 0.2)
              (bind _output_get_4 (Variables|Default|SetLongActCool (+ (Variables|Default|GetLongActCool) 0.5)))
              (Utilities|FlowControl|Delay 0.5)
              (if (== _output_get_4 1.0)
                (Variables|Default|SetLongActVar true)
                (Utilities|FlowControl|Delay 0.2)
                (goto _label_3))))
          (:then_1
            (Variables|Default|Setwhat2 true)))))))

(event EventBeginPlay)

(event EventSetLoadInventorytoPlayer
  (params (Player :type Beat%20Night%20Player%20Object%20Reference))
  (bind _loadgameinstance (Variables|Default|GetLoadGameInstance))
  (bind _weapondata (Variables|/Script/UE4_BeatNight.BeatNightSaveGame|GetWeaponData _loadgameinstance))
  (bind (_weaponindex _weaponammo _weapontypearr _weaponnamearr _weaponswordlevelarr) (Utilities|Struct|BreakWeaponData _weapondata))
  ;[1 1 1] 인벤토리 불러오기
  (Variables|Default|SetPlayer (.AsBP%20Player (Utilities|Casting|CastToBP_Player Player)))
  (|SetArray _weaponindex _weaponammo _weapontypearr _weaponnamearr _weaponswordlevelarr)
  (for (_array_element _array_index) (Variables|Inventory|GetLoadWeaponType)
    (switch Utilities|FlowControl|Switch|SwitchonEWeaponType _array_element
      (:EWT_Sword
        (|Sword _array_index))
      (:EWT_Gun
        (switch Utilities|FlowControl|Switch|SwitchonEWeaponName (Utilities|Array|Get(acopy) (Variables|Inventory|GetLoadWeaponName) _array_index)
          (:EWN_Anaconda
            (|Anaconda "/Game/00_BeatNight/Weapons/Guns/Anaconda/BP_Anaconda.BP_Anaconda_C" _array_index))
          (:EWN_ColtDouble
            (|ColtDouble "/Game/00_BeatNight/Weapons/Guns/ColtDouble/BP_ColtDouble.BP_ColtDouble_C" _array_index))
          (:EWN_Remington
            (|Remington "/Game/00_BeatNight/Weapons/Guns/Remington/BP_Remington.BP_Remington_C" _array_index))
          (:EWN_ShotGun
            (|ShotGun "/Game/00_BeatNight/Weapons/Guns/Shotgun/BP_Shotgun.BP_Shotgun_C" _array_index))
          (:EWN_Winchester
            (|Winchester "/Game/00_BeatNight/Weapons/Guns/Winchester/BP_Winchester.BP_Winchester_C" _array_index))))
      (:EWT_Rope
        (|Rope "/Game/00_BeatNight/Weapons/RopeGun/RopeGun.RopeGun_C" _array_index))))
  (Variables|/Script/UE4_BeatNight.BeatNightPlayer|SetInventory Player (Variables|Default|GetResultInventory)))

(fn ConstructionScript)

(fn SpawnWeapon
  (params (Weapon :type Weapon%20Object%20Reference))
  (bind _returnvalue (Game|SpawnActorfromClass (Utilities|GetClass Weapon) (Math|Transform|MakeTransform "0, 0, 0") "AlwaysSpawn" 0 0))
  (Utilities|Array|Add (Variables|Default|GetResultInventory) _returnvalue))