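; Game mode for BeatNight that plays the level 1 music track on BeginPlay and generates short and long rhythm timing windows.
; Tick launches two self-repeating Delay loops, each only once via a guard flag.
; The loops count up cooldown values and briefly raise ShortActVar and LongActVar, with the long window recurring at half the short one's rate.
; Timing comes from the delays alone, not from audio playback position.
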(event EventTick
  (params (DeltaSeconds :type Float%20%28single-precision%29))
  (Utilities|FlowControl|Sequence
    (:then_0
      (if (not (Variables|Default|Getwhat))
        (Utilities|FlowControl|Sequence
          (:then_0
            (bind _output_get (Variables|Default|SetShortActCool 0.0 :!label _label))
            (if (< _output_get 1.0)
              (Variables|Default|SetShortActVar false)
              (Utilities|FlowControl|Delay 0.5 :!label _label_2)
              (bind _output_get_2 (Variables|Default|SetShortActCool (+ (Variables|Default|GetShortActCool) 1.0)))
              (if (== _output_get_2 1.0)
                (Variables|Default|SetShortActVar true)
                (Utilities|FlowControl|Delay 0.2)
                (goto _label)
                (else
                  (goto _label_2)))))
          (:then_1
            (Variables|Default|Setwhat true)))))
    (:then_1
      ;[1 1 1] 긴 리듬
      (if (not (Variables|Default|Getwhat2))
        (Utilities|FlowControl|Sequence
          (:then_0
            (bind _output_get_3 (Variables|Default|SetLongActCool 0.0 :!label _label_3))
            (if (< _output_get_3 1.0)
              (Variables|Default|SetLongActVar false)
              (Utilities|FlowControl|Delay 0.5 :!label _label_4)
              (Variables|Default|SetLongActCool (+ (Variables|Default|GetLongActCool) 0.5))
              (Utilities|FlowControl|Delay 0.2)
              (Variables|Default|SetLongActVar false)
              (Utilities|FlowControl|Delay 0.5)
              (bind _output_get_4 (Variables|Default|SetLongActCool (+ (Variables|Default|GetLongActCool) 0.5)))
              (if (== _output_get_4 1.0)
                (Variables|Default|SetLongActVar true)
                (Utilities|FlowControl|Delay 0.2)
                (goto _label_3)
                (else
                  (goto _label_4)))))
          (:then_1
            (Variables|Default|Setwhat2 true)))))))

(event EventBeginPlay
  (Audio|PlaySound2D "/Game/00_BeatNight/LV1__바_Speed1_25x_.LV1__바_Speed1_25x_" 1.0 1.0 0.0 0 0))

(fn ConstructionScript)