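; BP_Defense is a defense item in BeatNight, offered for coins through a purchase button widget.
; Its SetWidgetCoinNum event casts the WidgetComponent's widget to W_PurchaseButton and fills in the coin cost, "Defense" name, defense amount, pickup sound and a self-reference as the item type.
; BeginPlay, overlap, Tick and the construction script are empty, and this graph contains no purchase or stat-change logic.
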(event EventBeginPlay)

(event Collision|EventActorBeginOverlap
  (params (OtherActor :type Actor%20Object%20Reference)))

(event EventTick
  (params (DeltaSeconds :type Float%20%28single-precision%29)))

(event EventSetWidgetCoinNum
  (bind _asw_purchase_button (Utilities|Casting|CastToW_PurchaseButton (UserInterface|GetWidget (Variables|Default|GetWidgetComponent))))
  (Variables|/Game/XMesh/Shieldver2/W_PurchaseButton.W_PurchaseButton_C|SetCoinNum _asw_purchase_button (Math|Conversions|ToInteger(Byte) (Variables|Default|GetItemCoin)))
  (Variables|/Game/XMesh/Shieldver2/W_PurchaseButton.W_PurchaseButton_C|SetItemName _asw_purchase_button "Defense")
  (Variables|/Game/XMesh/Shieldver2/W_PurchaseButton.W_PurchaseButton_C|SetAmount _asw_purchase_button (Variables|Default|GetDefenseAmount))
  (Variables|/Game/XMesh/Shieldver2/W_PurchaseButton.W_PurchaseButton_C|SetSound _asw_purchase_button (Variables|Default|GetPickupSound))
  (Variables|/Game/XMesh/Shieldver2/W_PurchaseButton.W_PurchaseButton_C|SetItemType _asw_purchase_button self))

(fn ConstructionScript)