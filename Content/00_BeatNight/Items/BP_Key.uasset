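; BP_Key is a key item with a purchase widget showing a coin price, built on a parent item class.
; On BeginPlay it runs the parent logic, then sets a fixed rotation on the actor when its item type is Normal.
; SetWidgetCoinNum fills the W_PurchaseButton in its widget component with the name "Key", a reference to itself and the item's coin cost as an integer.
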(event EventBeginPlay
  (|CallParentFunction)
  (if (Utilities|Enum|Equal(Enum) (Variables|Default|GetItemType) "EIT_Normal")
    (Transformation|SetActorRotation "50.000000, 0,90.000000")))

(event Collision|EventActorBeginOverlap
  (params (OtherActor :type Actor%20Object%20Reference)))

(event EventTick
  (params (DeltaSeconds :type Float%20%28single-precision%29)))

(event EventSetWidgetCoinNum
  (bind _asw_purchase_button (Utilities|Casting|CastToW_PurchaseButton (UserInterface|GetWidget (Variables|Default|GetWidgetComponent))))
  (Variables|/Game/XMesh/Shieldver2/W_PurchaseButton.W_PurchaseButton_C|SetItemName _asw_purchase_button "Key")
  (Variables|/Game/XMesh/Shieldver2/W_PurchaseButton.W_PurchaseButton_C|SetItemType _asw_purchase_button self)
  (Variables|/Game/XMesh/Shieldver2/W_PurchaseButton.W_PurchaseButton_C|SetCoinNum _asw_purchase_button (Math|Conversions|ToInteger(Byte) (Variables|Default|GetItemCoin))))

(fn ConstructionScript)