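; Gacha box that spawns a random item above itself when a player overlaps its area, a temporary trigger until a lever pull replaces it.
; Each overlap reseeds a random stream from the current milliseconds and rolls one number.
; SetGachaSpawnItem tests that roll against weighted ranges covering health packs, sword upgrade, dual blade, guns and defense boosts.
; Dual blade and defense spawns get their level or amount set afterward.
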(event OnComponentBeginOverlap(AreaSphere)
  (params (OverlappedComponent :type Primitive%20Component%20Object%20Reference) (OtherActor :type Actor%20Object%20Reference) (OtherComp :type Primitive%20Component%20Object%20Reference) (OtherBodyIndex :type Integer) (bFromSweep :type Boolean) (SweepResult :type Hit%20Result%20Structure%20%28by%20ref%29))
  ;[1 1 1] 임시 > 차후 레버 당기기로 변경예정
  (bind _asbp_player (Utilities|Casting|CastToBP_Player OtherActor))
  (Utilities|IsValid _asbp_player
    (:Is%20Valid
      ;[1 1 1] 랜덤값 지정
      (Math|Random|SetRandomStreamSeed (Variables|Default|GetRandomStream) (Math|Random|RandomInteger (Math|DateTime|GetMillisecond (Math|DateTime|Now))))
      (Variables|Default|SetRandomInt (Math|Random|RandomIntegerinRangefromStream 0 100 (Variables|Default|GetRandomStream)))
      (if (Variables|Default|GetIsSpawn)
        (Utilities|FlowControl|Sequence
          (:then_0
            ;[1 1 1] 30% 확률 포션
            (CallFunction|SetGachaSpawnItem 0 30 "/Game/00_BeatNight/Items/BP_HealthPack.BP_HealthPack_C"))
          (:then_1
            ;[1 1 1] 10% 확률 칼 업그레이드
            (CallFunction|SetGachaSpawnItem 30 40 "/Game/00_BeatNight/Items/BP_SwordUpgrade.BP_SwordUpgrade_C"))
          (:then_2
            ;[1 1 1] 3% 확률 듀얼블레이드
            (CallFunction|SetGachaSpawnItem 40 43 "/Game/00_BeatNight/Weapons/Swords/BP_Sword.BP_Sword_C")
            (bind _asbp_sword (Utilities|Casting|CastToBP_Sword (Variables|Default|GetItemClass)))
            (Utilities|IsValid _asbp_sword
              (:Is%20Valid
                (Variables|/Script/UE4_BeatNight.Weapon_Sword|SetSwordType _asbp_sword "EST_Level4")
                (Class|WeaponSword|SetWeaponDataTable _asbp_sword))))
          (:then_3
            ;[1 1 1] 16% 확률 레밍턴
            (CallFunction|SetGachaSpawnItem 43 59 "/Game/00_BeatNight/Weapons/Guns/Remington/BP_Remington.BP_Remington_C"))
          (:then_4
            ;[1 1 1] 12% 확률 콜트
            (CallFunction|SetGachaSpawnItem 59 71 "/Game/00_BeatNight/Weapons/Guns/ColtDouble/BP_ColtDouble.BP_ColtDouble_C"))
          (:then_5
            ;[1 1 1] 9% 확률 아나콘다
            (CallFunction|SetGachaSpawnItem 71 80 "/Game/00_BeatNight/Weapons/Guns/Anaconda/BP_Anaconda.BP_Anaconda_C"))
          (:then_6
            ;[1 1 1] 8% 확률 윈체스터
            (CallFunction|SetGachaSpawnItem 80 88 "/Game/00_BeatNight/Weapons/Guns/Winchester/BP_Winchester.BP_Winchester_C"))
          (:then_7
            ;[1 1 1] 7% 확률 샷건
            (CallFunction|SetGachaSpawnItem 88 95 "/Game/00_BeatNight/Weapons/Guns/Shotgun/BP_Shotgun.BP_Shotgun_C"))
          (:then_8
            ;[1 1 1] 5% 확률 방어력 증가
            (CallFunction|SetGachaSpawnItem 95 100 "/Script/UE4_BeatNight.Item_Defense")
            (bind _asitem_defense (Utilities|Casting|CastToItem_Defense (Variables|Default|GetItemClass)))
            (Utilities|IsValid _asitem_defense
              (:Is%20Valid
                (Variables|/Script/UE4_BeatNight.Item_Defense|SetDefenseAmount _asitem_defense 2e+01)))))))))

(event EventBeginPlay
  (bind _returnvalue (Transformation|GetActorLocation))
  (|CallParentFunction)
  ;[1 1 1] 스폰위치
  (Variables|Default|SetSpawnLocation (Math|Vector|MakeVector (.x _returnvalue) (.y _returnvalue) (+ (.z _returnvalue) 6e+01))))

(fn ConstructionScript)

(fn SetGachaSpawnItem
  (params (Min :type Integer) (Max :type Integer) (GachaItem :type Item%20Class%20Reference))
  (bind _randomint (Variables|Default|GetRandomInt))
  (if (and (>= _randomint Min) (< _randomint Max))
    ;[1 1 1] 결과가 True면 변수를 False로 변환해 함수를 타지 않게
    (Variables|Default|SetIsSpawn false)
    (bind _output_get (Variables|Default|SetGachaItem GachaItem))
    (bind _returnvalue (Game|SpawnActorfromClass _output_get (Math|Transform|MakeTransform (Variables|Default|GetSpawnLocation)) "AlwaysSpawn" 0 0))
    (Variables|Default|SetItemClass _returnvalue)
    ;[1 1 1] 다시 스폰될 수 있도록 변경
    (Variables|Default|SetIsSpawn true)))