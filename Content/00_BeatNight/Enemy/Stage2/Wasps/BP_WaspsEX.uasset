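; Stage 2 flying wasp enemy pawn that patrols, chases the player and plays an attack montage.
; Two looping timers replace Tick: one detects the player via view-cone dot check and Pawn-only line trace, the other drives movement by flying mode.
; Patrol cycles tagged actors, Aggro pursues the last seen location, and LookingForPlayer counts ticks there before returning to patrol.
; Movement uses FloatingPawnMovement with interpolated rotation; a Dying flag halts the logic.
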(event Custom|MovementTick
  ;[1 1 1] Movement Tick
  (if (not (Variables|Default|GetbDying))
    (switch Utilities|FlowControl|Switch|SwitchonE_AggroFlyingMode (Variables|Move|GetFlyingMode)
      (:NewEnumerator0
        (CallFunction|PatrolMovement))
      (:NewEnumerator1
        (CallFunction|AggroMovement)
        (Utilities|FlowControl|Delay (Variables|Default|GetDelayAttackTime))
        (Animation|PlayAnimMontage "/Game/00_BeatNight/Enemy/Stage2/Wasps/Animations/AttackMontage.AttackMontage" 1.0 "None"))
      (:NewEnumerator2
        (CallFunction|LFPMovement)))))

(event Custom|CheckForPlayerTick
  ;[1 1 1] CFP(CheckForPlayer)
  (if (not (Variables|Default|GetbDying))
    (bind (_findplayer_ _location) (CallFunction|TraceforPlayer))
    (if _findplayer_
      (Variables|Aggro|SetLastSawPlayerLocation _location)
      (Variables|Move|SetFlyingMode "NewEnumerator1")
      (else
        (switch Utilities|FlowControl|Switch|SwitchonE_AggroFlyingMode (Variables|Move|GetFlyingMode)
          (:NewEnumerator1
            (Variables|Move|SetFlyingMode "NewEnumerator2")
            (Variables|Aggro|SetLookingForPlayerCounter 0)))))))

(event Custom|PatrolMovement
  (bind _patrolpoints (Variables|Patrol|GetPatrolPoints))
  (bind _patrolindex (Variables|Patrol|GetPatrolIndex))
  (bind _output (Utilities|Array|Get(acopy) _patrolpoints _patrolindex))
  ;[1 1 1] Patrol
  (if (not (Variables|Default|GetbDying))
    (if (Variables|Patrol|GetCanPatrol)
      (if (< (Transformation|GetDistanceTo self _output) (Variables|Patrol|GetPatrolAcceptanceRadius))
        (CallFunction|GetNextPatrolLocation)
        (else
          (CallFunction|DoMovementTick true true (Transformation|GetActorLocation _output)))))))

(event Custom|AggroMovement
  (if (not (Variables|Default|GetbDying))
    (if (> (Math|Vector|VectorLength (- (Transformation|GetActorLocation) (Variables|Aggro|GetLastSawPlayerLocation))) (Variables|Aggro|GetAggroAcceptanceRadius))
      (CallFunction|DoMovementTick true true (Variables|Aggro|GetLastSawPlayerLocation))
      (else
        (CallFunction|DoMovementTick false true (Variables|Aggro|GetLastSawPlayerLocation))
        (Variables|/Script/Engine.MovementComponent|SetVelocity (Variables|Default|GetFloatingPawnMovement) "0, 0, 0")))))

(event Custom|LFPMovement
  (if (not (Variables|Default|GetbDying))
    (if (> (Math|Vector|VectorLength (- (Transformation|GetActorLocation) (Variables|Aggro|GetLastSawPlayerLocation))) (Variables|Aggro|GetAggroAcceptanceRadius))
      (CallFunction|DoMovementTick true true (Variables|Aggro|GetLastSawPlayerLocation))
      (else
        (Variables|/Script/Engine.MovementComponent|SetVelocity (Variables|Default|GetFloatingPawnMovement) "0, 0, 0")
        (bind _result (Math|Integer|IncrementInt (Variables|Aggro|GetLookingForPlayerCounter))
          (:%20%20
            (if (> _result (Variables|Aggro|GetMaxLFP))
              (Variables|Move|SetFlyingMode "NewEnumerator0"))))))))

(event Custom|DoMovementTick
  (params (DoFowardMovement :type Boolean) (DoRotation :type Boolean) (Location :type Vector))
  ;[1 1 1] Movement
  (if (not (Variables|Default|GetbDying))
    (Utilities|FlowControl|Sequence
      (:then_0
        (if DoFowardMovement
          (Class|PawnMovementComponent|AddInputVector (Variables|Default|GetFloatingPawnMovement) (CallFunction|FowardSpeed) false)))
      (:then_1
        (if DoRotation
          (Transformation|SetActorRotation (CallFunction|ForSmoothRotation Location)))))))

(event EventBeginPlay
  (|CallParentFunction)
  (CallFunction|CheckCanPatrol)
  ;[1 1 1] Movement Tick
  (bind _returnvalue (Utilities|Time|SetTimerbyEvent (delegate Custom|MovementTick) (Variables|Move|GetMovementTickRate) true))
  (Variables|Move|SetMovementTimer _returnvalue)
  ;[1 1 1] CFP(CheckForPlayer)
  (bind _returnvalue_2 (Utilities|Time|SetTimerbyEvent (delegate Custom|CheckForPlayerTick) (Variables|CheckforPlayer|GetCheckForPlayerTickRate) true))
  (Variables|CheckForPlayer|SetCheckForPlayerTimer _returnvalue_2))

(fn ConstructionScript
  (|CallParentFunction)
  (bind _outactors (Actor|GetAllActorswithTag (Variables|Default|GetPatrolTagName)))
  (Variables|Patrol|SetPatrolPoints _outactors))

(fn FowardSpeed
  (bind _aggromovespeed (Variables|Aggro|GetAggroMoveSpeed))
  (return (* (Transformation|GetActorForwardVector) (Utilities|Select :Index (Variables|Move|GetFlyingMode) :Option%200 (Variables|Patrol|GetPatrolMoveSpeed) :Option%201 _aggromovespeed :Option%202 _aggromovespeed))))

(fn ForSmoothRotation
  (params (Location :type Vector))
  (bind _aggrorinterpspeed (Variables|Aggro|GetAggroRInterpSpeed))
  (return (Math|Interpolation|RInterpTo (Transformation|GetActorRotation) (Math|Conversions|RotationFromXVector (Math|Vector|Normalize (- Location (Transformation|GetActorLocation)))) (Variables|Move|GetMovementTickRate) (Utilities|Select :Index (Variables|Move|GetFlyingMode) :Option%200 (Variables|Aggro|GetPatrolRInterpSpeed) :Option%201 _aggrorinterpspeed :Option%202 _aggrorinterpspeed))))

(fn CheckCanPatrol
  (if (Variables|Default|GetbDying)
    (Variables|Patrol|SetCanPatrol false)
    (elif (> (Utilities|Array|Length (Variables|Patrol|GetPatrolPoints)) 0)
      (Variables|Patrol|SetCanPatrol false)
      (for _array_element (Variables|Patrol|GetPatrolPoints)
        (Utilities|IsValid _array_element
          (:Is%20Not%20Valid
            (Math|Integer|IncrementInt (LocalVariables|GetInvalidIndexes)))))
      (Variables|Patrol|SetCanPatrol (not (== (LocalVariables|GetInvalidIndexes) (Utilities|Array|Length (Variables|Patrol|GetPatrolPoints))))))))

(fn GetNextPatrolLocation
  (if (not (Variables|Default|GetbDying))
    (bind _output_get (Variables|Patrol|SetPatrolIndex (Math|Integer|SelectInt 0 (+ (Variables|Patrol|GetPatrolIndex) 1) (== (+ (Variables|Patrol|GetPatrolIndex) 1) (Utilities|Array|Length (Variables|Patrol|GetPatrolPoints)))) :!label _label))
    (Utilities|IsValid (Utilities|Array|Get(acopy) (Variables|Patrol|GetPatrolPoints) _output_get)
      (:Is%20Not%20Valid
        (goto _label)))))

(fn TraceforPlayer
  (bind _returnvalue (Transformation|GetActorLocation))
  (bind _returnvalue_2 (Game|Player|GetPlayerPawn 0))
  (bind _arrowcomp (Variables|Default|GetArrowComp))
  (bind _returnvalue_3 (Transformation|GetWorldLocation _arrowcomp))
  (bind _asbp_player (Utilities|Casting|CastToBP_Player _returnvalue_2))
  (bind _returnvalue_4 (Transformation|GetActorLocation _asbp_player))
  (bind _returnvalue_5 (- _returnvalue_4 _returnvalue))
  (bind _returnvalue_6 (Math|Vector|Normalize _returnvalue_5))
  (if (Variables|Default|GetbDying)
    (return false "0, 0, 0")
    (elif (> (Math|Vector|DotProduct (Math|Vector|GetForwardVector (Variables|Default|GetArrowComp)) _returnvalue_6) (Variables|CheckforPlayer|GetFindPlayerDot))
      (bind _outhit (Collision|LineTraceForObjects _returnvalue_3 (+ _returnvalue_3 (* _returnvalue_6 (Variables|CheckforPlayer|GetPlayerTraceDistance))) (Utilities|Array|MakeArray "ObjectTypeQuery3") false 0 (select (Variables|CheckforPlayer|GetTraceDebug) "None" "None")))
      (if (.bBlockingHit (Collision|BreakHitResult _outhit))
        (return (== (.AsBP%20Player (Utilities|Casting|CastToBP_Player (Game|Player|GetPlayerPawn 0))) (.HitActor (Collision|BreakHitResult _outhit))) (.Location (Collision|BreakHitResult _outhit)))
        (else
          (return false "0, 0, 0")))
      (else
        (return false "0, 0, 0")))))