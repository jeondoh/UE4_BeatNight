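; BP_Remington is a Remington gun actor that can be picked up, dropped and fired.
; Pickup turns off mesh physics, attaches the root to the supplied component and snaps the mesh to a fixed relative grip transform.
; Drop re-enables physics and detaches the actor.
; FireRemington runs a debug-drawn Visibility line trace forward from the Arrow component, without using the hit result.
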(event EventBeginPlay)

(event Collision|EventActorBeginOverlap
  (params (OtherActor :type Actor%20Object%20Reference)))

(event EventTick
  (params (DeltaSeconds :type Float%20%28single-precision%29)))

(event EventPickup
  (params (AttachTo :type Scene%20Component%20Object%20Reference))
  (Physics|SetSimulatePhysics (Variables|Default|GetStaticMeshComponent) false)
  (Transformation|AttachComponentToComponent (VehicleSound|GetRootComponent) AttachTo "None" "KeepWorld" "KeepWorld" "KeepWorld" false)
  (Transformation|SetRelativeLocationAndRotation (Variables|Default|GetStaticMeshComponent) "-6.000000,0.000000,-17.000000" "90.000000,0.000000,180.000000" false false))

(event EventDrop
  (Physics|SetSimulatePhysics (Variables|Default|GetStaticMeshComponent) true)
  (Transformation|DetachFromActor "KeepWorld" "KeepWorld" "KeepWorld"))

(fn ConstructionScript)

(fn FireRemington
  (bind _arrow (Variables|Default|GetArrow))
  (bind _returnvalue (Transformation|GetWorldLocation _arrow))
  (Collision|LineTraceByChannel _returnvalue (+ _returnvalue (* (Math|Vector|GetForwardVector (Transformation|GetWorldRotation _arrow)) 3e+03)) "TraceTypeQuery1" false 0 "ForDuration"))