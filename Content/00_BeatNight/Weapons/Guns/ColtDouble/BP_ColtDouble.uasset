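; BP_ColtDouble is a VR handgun that motion controllers pick up and drop, toggling physics, attachment, glow meshes and the game mode's IsShort flag.
; FireColtDouble runs an ammo check, spawns muzzle flash and shell ejection emitters at sockets, then has BP_Player trace forward from the Arrow to damage enemies.
; An empty magazine plays a miss sound and clears CanFire, which is returned to the caller rather than gating the shot inside the function.
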(event OnComponentBeginOverlap(Glow)
  (params (OverlappedComponent :type Primitive%20Component%20Object%20Reference) (OtherActor :type Actor%20Object%20Reference) (OtherComp :type Primitive%20Component%20Object%20Reference) (OtherBodyIndex :type Integer) (bFromSweep :type Boolean) (SweepResult :type Hit%20Result%20Structure%20%28by%20ref%29))
  (Utilities|Casting|CastToBP_MotionController OtherActor)
  (Rendering|SetVisibility (Variables|Default|GetGlow) true false))

(event OnComponentEndOverlap(Glow)
  (params (OverlappedComponent :type Primitive%20Component%20Object%20Reference) (OtherActor :type Actor%20Object%20Reference) (OtherComp :type Primitive%20Component%20Object%20Reference) (OtherBodyIndex :type Integer))
  (Utilities|Casting|CastToBP_MotionController OtherActor)
  (Rendering|SetVisibility (Variables|Default|GetGlow) false false))

(event EventBeginPlay)

(event Collision|EventActorBeginOverlap
  (params (OtherActor :type Actor%20Object%20Reference)))

(event EventTick
  (params (DeltaSeconds :type Float%20%28single-precision%29)))

(event EventPickup
  (params (AttachTo :type Scene%20Component%20Object%20Reference))
  (Physics|SetSimulatePhysics (Variables|Default|GetStaticMeshComponent) false)
  (Transformation|AttachComponentToComponent (VehicleSound|GetRootComponent) AttachTo "None" "KeepWorld" "KeepWorld" "KeepWorld" false)
  (Transformation|SetRelativeLocationAndRotation (Variables|Default|GetStaticMeshComponent) "-16.000000,0.000000,-16.000000" "0.000000,-90.000000,90.000000" false false)
  (bind _asbp_beat_night_game_mode_base (Utilities|Casting|CastToBP_BeatNightGameModeBase (Game|GetGameMode)))
  (Variables|/Game/00_BeatNight/GameMode/BP_BeatNightGameModeBase.BP_BeatNightGameModeBase_C|SetIsShort _asbp_beat_night_game_mode_base true)
  (Rendering|SetVisibility (Variables|Default|GetNoneGrapGlow) false false))

(event EventDrop
  (Physics|SetSimulatePhysics (Variables|Default|GetStaticMeshComponent) true)
  (Transformation|DetachFromActor "KeepWorld" "KeepWorld" "KeepWorld")
  (bind _asbp_beat_night_game_mode_base (Utilities|Casting|CastToBP_BeatNightGameModeBase (Game|GetGameMode)))
  (Variables|/Game/00_BeatNight/GameMode/BP_BeatNightGameModeBase.BP_BeatNightGameModeBase_C|SetIsShort _asbp_beat_night_game_mode_base false)
  (Rendering|SetVisibility (Variables|Default|GetNoneGrapGlow) true false))

(fn ConstructionScript)

(fn FireColtDouble
  (bind _arrow (Variables|Default|GetArrow))
  (bind _returnvalue (Transformation|GetWorldLocation _arrow))
  (|AmmoCheck
    (:%20%20
      (|SpawnGunFireParticle)
      (bind _asbp_player (Utilities|Casting|CastToBP_Player (Game|Player|GetPlayerPawn 0)))
      (Utilities|IsValid _asbp_player
        (:Is%20Valid
          (Class|BeatNightPlayer|TraceEnemytoDamage _asbp_player _returnvalue (+ _returnvalue (* (Math|Vector|GetForwardVector (Transformation|GetWorldRotation _arrow)) 3e+03)) (Math|Conversions|ToFloat(Integer) (Variables|Default|GetWeaponDamage)))
          (return (Variables|Default|GetbCanFire)))))))