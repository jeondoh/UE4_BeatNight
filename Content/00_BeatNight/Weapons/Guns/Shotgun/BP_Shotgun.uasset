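; VR shotgun for BeatNight that motion controllers pick up, drop and fire as a multi-pellet hitscan weapon.
; Pickup snaps it to the first hand, while Drop restores physics; both update the game mode's IsLong flag and glow meshes.
; FireShotgun gates on ammo, playing a miss sound when empty, then spawns muzzle, casing and smoke particles.
; Each pellet takes a random spread from the Arrow, with damage traced through BP_Player.
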(event OnComponentBeginOverlap(StaticMeshComponent)
  (params (OverlappedComponent :type Primitive%20Component%20Object%20Reference) (OtherActor :type Actor%20Object%20Reference) (OtherComp :type Primitive%20Component%20Object%20Reference) (OtherBodyIndex :type Integer) (bFromSweep :type Boolean) (SweepResult :type Hit%20Result%20Structure%20%28by%20ref%29))
  (Utilities|Casting|CastToBP_MotionController OtherActor)
  (Rendering|SetVisibility (Variables|Default|GetGrabGlow) true false))

(event OnComponentEndOverlap(StaticMeshComponent)
  (params (OverlappedComponent :type Primitive%20Component%20Object%20Reference) (OtherActor :type Actor%20Object%20Reference) (OtherComp :type Primitive%20Component%20Object%20Reference) (OtherBodyIndex :type Integer))
  (Utilities|Casting|CastToBP_MotionController OtherActor)
  (Rendering|SetVisibility (Variables|Default|GetGrabGlow) false false))

(event EventPickup
  (params (AttachTo :type Scene%20Component%20Object%20Reference))
  (bind _returnvalue (Transformation|GetWorldTransform AttachTo))
  (Components|MoveComponentTo AttachTo (.location _returnvalue) (.rotation _returnvalue) false false 0.2 false)
  (if (not (Variables|디폴트|GetFirstHandAttached))
    (Physics|SetSimulatePhysics (Variables|Default|GetStaticMeshComponent) false)
    (Transformation|AttachComponentToComponent (VehicleSound|GetRootComponent) AttachTo "None" "SnapToTarget" "SnapToTarget" "KeepWorld" false)
    (Transformation|SetRelativeLocationAndRotation (Variables|Default|GetStaticMeshComponent) "-17.000000,0.000000,-32.000000" (Variables|디폴트|GetOneHandRotation) false false)
    (Variables|디폴트|SetFirstHandAttached true)
    (Variables|디폴트|SetSecondHandTracking false)
    (Variables|디폴트|SetFirstHand AttachTo)
    (bind _asbp_beat_night_game_mode_base (Utilities|Casting|CastToBP_BeatNightGameModeBase (Game|GetGameMode)))
    (Variables|/Game/00_BeatNight/GameMode/BP_BeatNightGameModeBase.BP_BeatNightGameModeBase_C|SetIsLong _asbp_beat_night_game_mode_base true)
    (Rendering|SetVisibility (Variables|Default|GetNoneGrabGlow) false false)
    (Rendering|SetVisibility (Variables|Default|GetGrabGlow) false false)))

(event EventDrop
  (Physics|SetSimulatePhysics (Variables|Default|GetStaticMeshComponent) true)
  (Transformation|DetachFromActor "KeepWorld" "KeepWorld" "KeepWorld")
  (Variables|디폴트|SetFirstHandAttached false)
  (Variables|디폴트|SetSecondHandTracking false)
  (bind _asbp_beat_night_game_mode_base (Utilities|Casting|CastToBP_BeatNightGameModeBase (Game|GetGameMode)))
  (Variables|/Game/00_BeatNight/GameMode/BP_BeatNightGameModeBase.BP_BeatNightGameModeBase_C|SetIsLong _asbp_beat_night_game_mode_base false)
  (Rendering|SetVisibility (Variables|Default|GetNoneGrabGlow) true false))

(fn ConstructionScript)

(fn FireShotgun
  (bind _arrow (Variables|Default|GetArrow))
  (bind _returnvalue (Transformation|GetWorldLocation _arrow))
  (bind _returnvalue_2 (Transformation|GetWorldRotation _arrow))
  (bind (_roll _pitch _yaw) (Math|Rotator|BreakRotator _returnvalue_2))
  (|AmmoCheck
    (:%20%20
      (|SpawnGunFireParticle)
      (for _index (range 0 5)
        (bind _asbp_player (Utilities|Casting|CastToBP_Player (Game|Player|GetPlayerPawn 0)))
        (Utilities|IsValid _asbp_player
          (:Is%20Valid
            (Class|BeatNightPlayer|TraceEnemytoDamage _asbp_player _returnvalue (+ _returnvalue (* (Math|Rotator|GetRotationXVector (Math|Rotator|MakeRotator _roll (+ _pitch (Math|Random|RandomFloatinRange -5.0 5.0)) (+ _yaw (Math|Random|RandomFloatinRange -8.0 8.0)))) 3e+03)) (Math|Conversions|ToFloat(Integer) (Variables|Default|GetWeaponDamage))))))
      (return (Variables|Default|GetbCanFire)))))