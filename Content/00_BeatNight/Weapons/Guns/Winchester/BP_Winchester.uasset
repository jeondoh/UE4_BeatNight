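; BP_Winchester is a two-handed motion-controller rifle for BeatNight.
; Pickup attaches it to the first hand and Drop restores physics; both update the game mode's IsLong flag.
; A second controller entering the trigger aims the gun by look-at pitch and yaw each Tick, with roll zeroed, and can keep aiming outside it depending on grip state.
; FireWinchester passes a forward line from the Arrow to BP_Player's damage trace.
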(event OnComponentBeginOverlap(SecondHandTrigger)
  (params (OverlappedComponent :type Primitive%20Component%20Object%20Reference) (OtherActor :type Actor%20Object%20Reference) (OtherComp :type Primitive%20Component%20Object%20Reference) (OtherBodyIndex :type Integer) (bFromSweep :type Boolean) (SweepResult :type Hit%20Result%20Structure%20%28by%20ref%29))
  (if (Variables|디폴트|GetFirstHandAttached)
    (bind _asbp_motion_controller (Utilities|Casting|CastToBP_MotionController OtherActor))
    (if (!= (Variables|/Game/VirtualRealityBP/Blueprints/BP_MotionController.BP_MotionController_C|GetMotionController _asbp_motion_controller) (Variables|디폴트|GetFirstHand))
      (Variables|디폴트|SetSecondHandTracking true)
      (Variables|디폴트|SetSecondHand (Variables|/Game/VirtualRealityBP/Blueprints/BP_MotionController.BP_MotionController_C|GetMotionController _asbp_motion_controller)))))

(event OnComponentEndOverlap(SecondHandTrigger)
  (params (OverlappedComponent :type Primitive%20Component%20Object%20Reference) (OtherActor :type Actor%20Object%20Reference) (OtherComp :type Primitive%20Component%20Object%20Reference) (OtherBodyIndex :type Integer))
  (if (Variables|디폴트|GetSecondHandTracking)
    (Utilities|IsValid (Variables|디폴트|GetSecondHand)
      (:Is%20Valid
        (if (and (.bSuccess (Utilities|Casting|CastToBP_MotionController (Components|GetOwner (Variables|디폴트|GetSecondHand)))) (Utilities|Enum|NotEqual(Enum) (Variables|/Game/VirtualRealityBP/Blueprints/BP_MotionController.BP_MotionController_C|GetGripState (.AsBP%20Motion%20Controller (Utilities|Casting|CastToBP_MotionController (Components|GetOwner (Variables|디폴트|GetSecondHand))))) "NewEnumerator2"))
          (Variables|디폴트|SetSecondHandTracking false :!label _label)
          (Variables|디폴트|SetSecondHand 0)
          (Transformation|SetRelativeRotation (Variables|Default|GetStaticMeshComponent) (Variables|디폴트|GetOneHandRotation) false false)))
      (:Is%20Not%20Valid
        (goto _label)))))

(event EventBeginPlay)

(event Collision|EventActorBeginOverlap
  (params (OtherActor :type Actor%20Object%20Reference)))

(event EventPickup
  (params (AttachTo :type Scene%20Component%20Object%20Reference))
  (if (not (Variables|디폴트|GetFirstHandAttached))
    (Physics|SetSimulatePhysics (Variables|Default|GetStaticMeshComponent) false)
    (Transformation|AttachComponentToComponent (VehicleSound|GetRootComponent) AttachTo "None" "SnapToTarget" "SnapToTarget" "KeepWorld" false)
    (Transformation|SetRelativeLocationAndRotation (Variables|Default|GetStaticMeshComponent) "-17.000000,0.000000,-31.000000" (Variables|디폴트|GetOneHandRotation) false false)
    (Variables|디폴트|SetFirstHandAttached true)
    (Variables|디폴트|SetSecondHandTracking false)
    (Variables|디폴트|SetFirstHand AttachTo)
    (bind _asbp_beat_night_game_mode_base (Utilities|Casting|CastToBP_BeatNightGameModeBase (Game|GetGameMode)))
    (Variables|/Game/00_BeatNight/GameMode/BP_BeatNightGameModeBase.BP_BeatNightGameModeBase_C|SetIsLong _asbp_beat_night_game_mode_base true)))

(event EventTick
  (params (DeltaSeconds :type Float%20%28single-precision%29))
  (bind _firsthand (Variables|디폴트|GetFirstHand))
  (bind _secondhand (Variables|디폴트|GetSecondHand))
  (bind _returnvalue (Transformation|GetWorldLocation _secondhand))
  (bind _returnvalue_2 (Transformation|GetWorldLocation _firsthand))
  (bind _returnvalue_3 (Math|Rotator|FindLookatRotation _returnvalue_2 _returnvalue))
  (bind (_roll _pitch _yaw) (Math|Rotator|BreakRotator _returnvalue_3))
  (if (and (Variables|디폴트|GetSecondHandTracking) (Utilities|IsValid (Variables|디폴트|GetSecondHand)))
    (Transformation|SetWorldRotation (Variables|Default|GetStaticMeshComponent) (Math|Rotator|MakeRotator 0.0 _pitch _yaw) false false)))

(event EventDrop
  (Physics|SetSimulatePhysics (Variables|Default|GetStaticMeshComponent) true)
  (Transformation|DetachFromActor "KeepWorld" "KeepWorld" "KeepWorld")
  (Variables|디폴트|SetFirstHandAttached false)
  (Variables|디폴트|SetSecondHandTracking false)
  (bind _asbp_beat_night_game_mode_base (Utilities|Casting|CastToBP_BeatNightGameModeBase (Game|GetGameMode)))
  (Variables|/Game/00_BeatNight/GameMode/BP_BeatNightGameModeBase.BP_BeatNightGameModeBase_C|SetIsLong _asbp_beat_night_game_mode_base false))

(fn ConstructionScript)

(fn FireWinchester
  (bind _arrow (Variables|Default|GetArrow))
  (bind _returnvalue (Transformation|GetWorldLocation _arrow))
  (bind _asbp_player (Utilities|Casting|CastToBP_Player (Game|Player|GetPlayerPawn 0)))
  (Utilities|IsValid _asbp_player
    (:Is%20Valid
      (Class|BeatNightPlayer|TraceEnemytoDamage _asbp_player _returnvalue (+ _returnvalue (* (Math|Vector|GetForwardVector (Transformation|GetWorldRotation _arrow)) 3e+03)) (Math|Conversions|ToFloat(Integer) (Variables|Default|GetWeaponDamage))))))