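; Winchester gun Blueprint for VR motion controllers that can be held with one or two hands.
; Pickup disables physics and attaches it to the first hand at a fixed offset; Drop restores physics and detaches.
; A different controller overlapping SecondHandTrigger starts two-handed aiming, with Tick pointing the mesh from first to second hand at zero roll.
; Leaving the trigger restores one-handed rotation, depending on the second hand's grip state.
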(event OnComponentBeginOverlap(SecondHandTrigger)
  (params (OverlappedComponent :type Primitive%20Component%20Object%20Reference) (OtherActor :type Actor%20Object%20Reference) (OtherComp :type Primitive%20Component%20Object%20Reference) (OtherBodyIndex :type Integer) (bFromSweep :type Boolean) (SweepResult :type Hit%20Result%20Structure%20%28by%20ref%29))
  (if (Variables|Default|GetFirstHandAttached)
    (bind _asbp_motion_controller (Utilities|Casting|CastToBP_MotionController OtherActor))
    (if (!= (Variables|/Game/VirtualRealityBP/Blueprints/BP_MotionController.BP_MotionController_C|GetMotionController _asbp_motion_controller) (Variables|Default|GetFirstHand))
      (Variables|Default|SetSecondHandTracking true)
      (Variables|Default|SetSecondHand (Variables|/Game/VirtualRealityBP/Blueprints/BP_MotionController.BP_MotionController_C|GetMotionController _asbp_motion_controller)))))

(event OnComponentEndOverlap(SecondHandTrigger)
  (params (OverlappedComponent :type Primitive%20Component%20Object%20Reference) (OtherActor :type Actor%20Object%20Reference) (OtherComp :type Primitive%20Component%20Object%20Reference) (OtherBodyIndex :type Integer))
  (if (Variables|Default|GetSecondHandTracking)
    (Utilities|IsValid (Variables|Default|GetSecondHand)
      (:Is%20Valid
        (if (and (.bSuccess (Utilities|Casting|CastToBP_MotionController (Components|GetOwner (Variables|Default|GetSecondHand)))) (Utilities|Enum|NotEqual(Enum) (Variables|/Game/VirtualRealityBP/Blueprints/BP_MotionController.BP_MotionController_C|GetGripState (.AsBP%20Motion%20Controller (Utilities|Casting|CastToBP_MotionController (Components|GetOwner (Variables|Default|GetSecondHand))))) "NewEnumerator2"))
          (Variables|Default|SetSecondHandTracking false :!label _label)
          (Variables|Default|SetSecondHand 0)
          (Transformation|SetRelativeRotation (Variables|Default|GetStaticMeshComponent) (Variables|Default|GetOneHandRotation) false false)))
      (:Is%20Not%20Valid
        (goto _label)))))

(event EventBeginPlay)

(event Collision|EventActorBeginOverlap
  (params (OtherActor :type Actor%20Object%20Reference)))

(event EventPickup
  (params (AttachTo :type Scene%20Component%20Object%20Reference))
  (if (not (Variables|Default|GetFirstHandAttached))
    (Physics|SetSimulatePhysics (Variables|Default|GetStaticMeshComponent) false)
    (Transformation|AttachComponentToComponent (VehicleSound|GetRootComponent) AttachTo "None" "SnapToTarget" "SnapToTarget" "KeepWorld" false)
    (Transformation|SetRelativeLocationAndRotation (Variables|Default|GetStaticMeshComponent) "-15.000000,0.000000,-35.000000" (Variables|Default|GetOneHandRotation) false false)
    (Variables|Default|SetFirstHandAttached true)
    (Variables|Default|SetSecondHandTracking false)
    (Variables|Default|SetFirstHand AttachTo)))

(event EventTick
  (params (DeltaSeconds :type Float%20%28single-precision%29))
  (bind _firsthand (Variables|Default|GetFirstHand))
  (bind _secondhand (Variables|Default|GetSecondHand))
  (bind _returnvalue (Transformation|GetWorldLocation _secondhand))
  (bind _returnvalue_2 (Transformation|GetWorldLocation _firsthand))
  (bind _returnvalue_3 (Math|Rotator|FindLookatRotation _returnvalue_2 _returnvalue))
  (bind (_roll _pitch _yaw) (Math|Rotator|BreakRotator _returnvalue_3))
  (if (and (Variables|Default|GetSecondHandTracking) (Utilities|IsValid (Variables|Default|GetSecondHand)))
    (Transformation|SetWorldRotation (Variables|Default|GetStaticMeshComponent) (Math|Rotator|MakeRotator 0.0 _pitch _yaw) false false)))

(event EventDrop
  (Physics|SetSimulatePhysics (Variables|Default|GetStaticMeshComponent) true)
  (Transformation|DetachFromActor "KeepWorld" "KeepWorld" "KeepWorld")
  (Variables|Default|SetFirstHandAttached false)
  (Variables|Default|SetSecondHandTracking false))

(fn ConstructionScript)