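; VR utility-belt inventory actor with six mesh slots that store the player's weapons.
; The belt and stowed weapons appear when a motion controller enters CollisionBox, then hide after a short delay once no controllers remain.
; A weapon-holding controller entering a slot triggers rumble, enlarges it and sets BP_Player's CanInventory and InventoryIndex via CheckInventory; leaving resets them.
; AttachToSlot and DetachToSlot snap weapons to slot meshes or release them.
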(event OnComponentBeginOverlap(CollisionBox)
  (params (OverlappedComponent :type Primitive%20Component%20Object%20Reference) (OtherActor :type Actor%20Object%20Reference) (OtherComp :type Primitive%20Component%20Object%20Reference) (OtherBodyIndex :type Integer) (bFromSweep :type Boolean) (SweepResult :type Hit%20Result%20Structure%20%28by%20ref%29))
  (Utilities|Casting|CastToBP_MotionController OtherActor)
  (CallFunction|ToggleAttachedActorsVisibility/collision false)
  (Variables|Default|SetOverlapped true))

(event OnComponentEndOverlap(CollisionBox)
  (params (OverlappedComponent :type Primitive%20Component%20Object%20Reference) (OtherActor :type Actor%20Object%20Reference) (OtherComp :type Primitive%20Component%20Object%20Reference) (OtherBodyIndex :type Integer))
  (Utilities|Casting|CastToBP_MotionController OtherActor)
  (Variables|Default|SetOverlapped false)
  (Utilities|FlowControl|Delay 0.4)
  (if (and (not (Variables|Default|GetOverlapped)) (< (Utilities|Array|Length (Collision|GetOverlappingActors OverlappedComponent "/Game/VirtualRealityBP/Blueprints/BP_MotionController.BP_MotionController_C" :!class /Script/Engine.PrimitiveComponent)) 1)) ; Check other hand is not still overlapping
    (CallFunction|ToggleAttachedActorsVisibility/collision true)))

(event OnComponentBeginOverlap(Slot5)
  (params (OverlappedComponent :type Primitive%20Component%20Object%20Reference) (OtherActor :type Actor%20Object%20Reference) (OtherComp :type Primitive%20Component%20Object%20Reference) (OtherBodyIndex :type Integer) (bFromSweep :type Boolean) (SweepResult :type Hit%20Result%20Structure%20%28by%20ref%29))
  (CallFunction|OverlaptoSlot OtherActor 4 (Variables|Default|GetOverlapped%20scale) OverlappedComponent))

(event OnComponentEndOverlap(Slot5)
  (params (OverlappedComponent :type Primitive%20Component%20Object%20Reference) (OtherActor :type Actor%20Object%20Reference) (OtherComp :type Primitive%20Component%20Object%20Reference) (OtherBodyIndex :type Integer))
  (CallFunction|OverlapEndtoSlot OtherActor)
  (Utilities|OverlapEndDelayed OverlappedComponent (Variables|Default|GetDefault%20scale)))

(event OnComponentBeginOverlap(Slot6)
  (params (OverlappedComponent :type Primitive%20Component%20Object%20Reference) (OtherActor :type Actor%20Object%20Reference) (OtherComp :type Primitive%20Component%20Object%20Reference) (OtherBodyIndex :type Integer) (bFromSweep :type Boolean) (SweepResult :type Hit%20Result%20Structure%20%28by%20ref%29))
  (CallFunction|OverlaptoSlot OtherActor 5 (Variables|Default|GetOverlapped%20scale) OverlappedComponent))

(event OnComponentEndOverlap(Slot6)
  (params (OverlappedComponent :type Primitive%20Component%20Object%20Reference) (OtherActor :type Actor%20Object%20Reference) (OtherComp :type Primitive%20Component%20Object%20Reference) (OtherBodyIndex :type Integer))
  (CallFunction|OverlapEndtoSlot OtherActor)
  (Utilities|OverlapEndDelayed OverlappedComponent (Variables|Default|GetDefault%20scale)))

(event OnComponentBeginOverlap(Slot1)
  (params (OverlappedComponent :type Primitive%20Component%20Object%20Reference) (OtherActor :type Actor%20Object%20Reference) (OtherComp :type Primitive%20Component%20Object%20Reference) (OtherBodyIndex :type Integer) (bFromSweep :type Boolean) (SweepResult :type Hit%20Result%20Structure%20%28by%20ref%29))
  (CallFunction|OverlaptoSlot OtherActor 0 (Variables|Default|GetOverlapped%20scale) OverlappedComponent))

(event OnComponentEndOverlap(Slot1)
  (params (OverlappedComponent :type Primitive%20Component%20Object%20Reference) (OtherActor :type Actor%20Object%20Reference) (OtherComp :type Primitive%20Component%20Object%20Reference) (OtherBodyIndex :type Integer))
  (CallFunction|OverlapEndtoSlot OtherActor)
  (Utilities|OverlapEndDelayed OverlappedComponent (Variables|Default|GetDefault%20scale)))

(event OnComponentBeginOverlap(Slot2)
  (params (OverlappedComponent :type Primitive%20Component%20Object%20Reference) (OtherActor :type Actor%20Object%20Reference) (OtherComp :type Primitive%20Component%20Object%20Reference) (OtherBodyIndex :type Integer) (bFromSweep :type Boolean) (SweepResult :type Hit%20Result%20Structure%20%28by%20ref%29))
  (CallFunction|OverlaptoSlot OtherActor 1 (Variables|Default|GetOverlapped%20scale) OverlappedComponent))

(event OnComponentEndOverlap(Slot2)
  (params (OverlappedComponent :type Primitive%20Component%20Object%20Reference) (OtherActor :type Actor%20Object%20Reference) (OtherComp :type Primitive%20Component%20Object%20Reference) (OtherBodyIndex :type Integer))
  (CallFunction|OverlapEndtoSlot OtherActor)
  (Utilities|OverlapEndDelayed OverlappedComponent (Variables|Default|GetDefault%20scale)))

(event OnComponentBeginOverlap(Slot3)
  (params (OverlappedComponent :type Primitive%20Component%20Object%20Reference) (OtherActor :type Actor%20Object%20Reference) (OtherComp :type Primitive%20Component%20Object%20Reference) (OtherBodyIndex :type Integer) (bFromSweep :type Boolean) (SweepResult :type Hit%20Result%20Structure%20%28by%20ref%29))
  (CallFunction|OverlaptoSlot OtherActor 2 (Variables|Default|GetOverlapped%20scale) OverlappedComponent))

(event OnComponentEndOverlap(Slot3)
  (params (OverlappedComponent :type Primitive%20Component%20Object%20Reference) (OtherActor :type Actor%20Object%20Reference) (OtherComp :type Primitive%20Component%20Object%20Reference) (OtherBodyIndex :type Integer))
  (CallFunction|OverlapEndtoSlot OtherActor)
  (Utilities|OverlapEndDelayed OverlappedComponent (Variables|Default|GetDefault%20scale)))

(event OnComponentBeginOverlap(Slot4)
  (params (OverlappedComponent :type Primitive%20Component%20Object%20Reference) (OtherActor :type Actor%20Object%20Reference) (OtherComp :type Primitive%20Component%20Object%20Reference) (OtherBodyIndex :type Integer) (bFromSweep :type Boolean) (SweepResult :type Hit%20Result%20Structure%20%28by%20ref%29))
  (CallFunction|OverlaptoSlot OtherActor 3 (Variables|Default|GetOverlapped%20scale) OverlappedComponent))

(event OnComponentEndOverlap(Slot4)
  (params (OverlappedComponent :type Primitive%20Component%20Object%20Reference) (OtherActor :type Actor%20Object%20Reference) (OtherComp :type Primitive%20Component%20Object%20Reference) (OtherBodyIndex :type Integer))
  (CallFunction|OverlapEndtoSlot OtherActor)
  (Utilities|OverlapEndDelayed OverlappedComponent (Variables|Default|GetDefault%20scale)))

(event EventBeginPlay
  (|CallParentFunction)
  (bind _asbp_player (Utilities|Casting|CastToBP_Player (Game|Player|GetPlayerPawn 0)))
  (Variables|Default|SetInventoryPlayer _asbp_player))

(fn ConstructionScript
  (|CallParentFunction)
  (Variables|Default|SetSlotMeshArr (Utilities|Array|MakeArray (Variables|Default|GetSlot1) (Variables|Default|GetSlot2) (Variables|Default|GetSlot3) (Variables|Default|GetSlot4) (Variables|Default|GetSlot5) (Variables|Default|GetSlot6))))

(fn ToggleAttachedActorsVisibility/collision
  (params (Hide%20actors :type Boolean))
  (for _array_element (Variables|Default|GetSlotMeshArr)
    (for _array_element_2 (Components|GetChildrenComponents _array_element true)
      (Utilities|FlowControl|Sequence
        (:then_0
          (Rendering|SetActorHiddenInGame (Components|GetOwner _array_element_2) Hide%20actors) ; Show weapon actors
          (Collision|SetActorEnableCollision (Components|GetOwner _array_element_2) (not Hide%20actors)) ; disable collision for all attached actors
          (Collision|SetActorEnableCollision true) ; enable utility belt collision
        )
        (:then_1
          (Rendering|SetActorHiddenInGame Hide%20actors))))))

(fn AttachtoSlot
  (params (Weapon :type Weapon%20Object%20Reference) (Index :type Integer))
  (switch int Index
    (:0
      (Variables|Default|SetStaticMesh (Variables|Default|GetSlot1)))
    (:1
      (Variables|Default|SetStaticMesh (Variables|Default|GetSlot2)))
    (:2
      (Variables|Default|SetStaticMesh (Variables|Default|GetSlot3)))
    (:3
      (Variables|Default|SetStaticMesh (Variables|Default|GetSlot4)))
    (:4
      (Variables|Default|SetStaticMesh (Variables|Default|GetSlot5)))
    (:5
      (Variables|Default|SetStaticMesh (Variables|Default|GetSlot6))))
  (Transformation|AttachComponentToComponent Weapon (Variables|Default|GetStaticMesh) "None" "SnapToTarget" "SnapToTarget" "KeepRelative" true))

(fn DetachtoSlot
  (params (Weapon :type Weapon%20Object%20Reference) (Index :type Integer))
  (Transformation|DetachFromActor Weapon "KeepWorld" "KeepWorld" "KeepRelative"))

(fn OverlaptoSlot
  (params (Object :type Object%20Object%20Reference) (InvenIndex :type Integer) (New%20Scale :type Vector) (Slot :type Scene%20Component%20Object%20Reference))
  (bind _inventoryplayer (Variables|Default|GetInventoryPlayer))
  (bind _asbp_motion_controller (Utilities|Casting|CastToBP_MotionController Object))
  (Utilities|IsValid _asbp_motion_controller
    (:Is%20Valid
      (bind _asweapon (Utilities|Casting|CastToWeapon (Variables|/Script/UE4_BeatNight.MontionActor|GetAttachedActor _asbp_motion_controller)))
      (Utilities|IsValid _asweapon
        (:Is%20Valid
          (Default|RumbleController _asbp_motion_controller 0.2)
          (Transformation|SetRelativeScale3D Slot New%20Scale)
          (CallFunction|ToggleAttachedActorsVisibility/collision false)
          (bind _returnvalue (Class|BeatNightPlayer|CheckInventory _inventoryplayer InvenIndex))
          (if _returnvalue
            (Variables|/Script/UE4_BeatNight.BeatNightPlayer|SetbCanInventory _inventoryplayer true)
            (Variables|/Script/UE4_BeatNight.BeatNightPlayer|SetInventoryIndex (Variables|Default|GetInventoryPlayer) InvenIndex)
            (else
              (Variables|/Script/UE4_BeatNight.BeatNightPlayer|SetbCanInventory _inventoryplayer false)
              (Variables|/Script/UE4_BeatNight.BeatNightPlayer|SetInventoryIndex (Variables|Default|GetInventoryPlayer) -1))))))))

(fn OverlapEndtoSlot
  (params (Object :type Object%20Object%20Reference))
  (bind _asbp_motion_controller (Utilities|Casting|CastToBP_MotionController Object))
  (Utilities|IsValid _asbp_motion_controller
    (:Is%20Valid
      (Variables|/Script/UE4_BeatNight.BeatNightPlayer|SetbCanInventory (Variables|Default|GetInventoryPlayer) false)
      (Variables|/Script/UE4_BeatNight.BeatNightPlayer|SetInventoryIndex (Variables|Default|GetInventoryPlayer) -1))))