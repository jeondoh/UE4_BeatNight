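; BP_PotalActor2 is a stage portal that moves the player to a target location behind a screen fade.
; Its NSPotal effect becomes visible on BeginPlay if CanMove is set, or when OpenDoor is called.
; PlayLevelSeq plays the SQFade sequence, waits briefly, starts it in reverse, teleports the player to MoveToLocation's X/Y at a fixed height, then clears CanMove.
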(event EventBeginPlay
  (|CallParentFunction)
  (if (Variables|Default|GetbCanMove)
    (Rendering|SetVisibility (Variables|Default|GetNS_Potal) true false)))

(event Collision|EventActorBeginOverlap
  (params (OtherActor :type Actor%20Object%20Reference)))

(event EventTick
  (params (DeltaSeconds :type Float%20%28single-precision%29)))

(event EventPlayLevelSeq
  (params (Player :type Beat%20Night%20Player%20Object%20Reference))
  (bind _movetolocation (Variables|Default|GetMoveToLocation))
  (bind _outactor (Sequencer|Player|CreateLevelSequencePlayer (Variables|Default|GetSQ_Fade)))
  (Sequencer|Player|Play (Variables|/Script/LevelSequence.LevelSequenceActor|GetSequencePlayer _outactor) :!class /Script/MovieScene.MovieSceneSequencePlayer)
  (Utilities|FlowControl|Delay 1.0)
  (Class|MovieSceneSequencePlayer|PlayReverse (Variables|/Script/LevelSequence.LevelSequenceActor|GetSequencePlayer _outactor))
  (Transformation|SetActorLocation Player (Math|Vector|MakeVector (.x _movetolocation) (.y _movetolocation) 5e+01) false false)
  (Variables|Default|SetbCanMove false))

(event EventOpenDoor
  (Rendering|SetVisibility (Variables|Default|GetNS_Potal) true false))

(fn ConstructionScript)