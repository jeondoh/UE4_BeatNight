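; BP_RopeGun is a grappling-hook gun that can be picked up, dropped and used to pull the player to a hit point.
; FireRope traces from the RopeDecoy player's camera against world objects to set the hook point, calling StopGrapple on a miss.
; Tick interpolates the GrappleLine cable to that point, then relaunches the character toward it every frame at distance-scaled velocity.
; StopGrapple resets the cable and launches the player upward.
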(event Custom|StopGrapple
  (bind _grappleline (Variables|Default|GetGrappleLine))
  (Variables|Default|SetHooked false)
  (Variables|Default|SetHookMoveFinished false)
  (Rendering|SetVisibility _grappleline false false)
  (Transformation|SetWorldLocation _grappleline "0, 0, 0" false false)
  (bind _asrope_decoy (Utilities|Casting|CastToRopeDecoy (Game|GetPlayerCharacter 0)))
  (Character|LaunchCharacter _asrope_decoy "0, 0,650.000000" false false))

(event EventBeginPlay
  (bind _grappleline (Variables|Default|GetGrappleLine))
  (Rendering|SetVisibility _grappleline false false)
  (Variables|/Script/CableComponent.CableComponent|SetCableLength _grappleline 0.0)
  (Variables|/Script/CableComponent.CableComponent|SetCableWidth _grappleline 6.0)
  (Variables|/Script/CableComponent.CableComponent|SetEndLocation _grappleline "0, 0, 0"))

(event Collision|EventActorBeginOverlap
  (params (OtherActor :type Actor%20Object%20Reference)))

(event EventPickup
  (params (AttachTo :type Scene%20Component%20Object%20Reference))
  (Physics|SetSimulatePhysics (Variables|Default|GetStaticMeshComponent) false)
  (Transformation|AttachComponentToComponent (VehicleSound|GetRootComponent) AttachTo "None" "KeepWorld" "KeepWorld" "KeepWorld" false)
  (Transformation|SetRelativeLocationAndRotation (Variables|Default|GetStaticMeshComponent) "-10.000000,0.000000,-20.000000" "0.000000,-90.000000,-90.000000" false false))

(event EventTick
  (params (DeltaSeconds :type Float%20%28single-precision%29))
  (bind _grappleline (Variables|Default|GetGrappleLine))
  (if (Variables|Default|GetHooked)
    (if (Variables|Default|GetHookMoveFinished)
      (CallFunction|MoveGrappledPlayer)
      (Transformation|SetWorldLocation _grappleline (Math|Interpolation|VInterpTo (Transformation|GetWorldLocation _grappleline) (Variables|Default|GetHookLocation) (Utilities|Time|GetWorldDeltaSeconds) 2.5e+02) false false)
      (else
        (bind _reachedlocation (CallFunction|MoveRope))
        (Variables|Default|SetHookMoveFinished _reachedlocation)))))

(event EventDrop
  (Physics|SetSimulatePhysics (Variables|Default|GetStaticMeshComponent) true)
  (Transformation|DetachFromActor "KeepWorld" "KeepWorld" "KeepWorld"))

(fn ConstructionScript)

(fn FireRope
  (bind _asrope_decoy (Utilities|Casting|CastToRopeDecoy (Game|GetPlayerCharacter 0)))
  (bind (_outhit _returnvalue) (Collision|LineTraceForObjects (Transformation|GetWorldLocation (Variables|/Game/00_BeatNight/RopeMove/RopeDecoy.RopeDecoy_C|GetCamera _asrope_decoy)) (+ (Transformation|GetWorldLocation (Variables|/Game/00_BeatNight/RopeMove/RopeDecoy.RopeDecoy_C|GetCamera _asrope_decoy)) (* (Math|Vector|GetForwardVector (Variables|/Game/00_BeatNight/RopeMove/RopeDecoy.RopeDecoy_C|GetCamera _asrope_decoy)) 5e+03)) (Utilities|Array|MakeArray "ObjectTypeQuery1" "ObjectTypeQuery2") false 0 "None"))
  (if _returnvalue
    (Variables|Default|SetHooked true)
    (Variables|Default|SetHookLocation (.Location (Collision|BreakHitResult _outhit)))
    (else
      (CallFunction|StopGrapple))))

(fn MoveRope
  (bind _grappleline (Variables|Default|GetGrappleLine))
  (bind _hooklocation (Variables|Default|GetHookLocation))
  (bind _returnvalue (Transformation|GetWorldLocation _grappleline))
  (Rendering|SetVisibility _grappleline true false)
  (if (<= (Math|Vector|VectorLength (- _returnvalue _hooklocation)) 1e+02)
    (return true)
    (else
      (Transformation|SetWorldLocation _grappleline (Math|Interpolation|VInterpTo _returnvalue _hooklocation (Utilities|Time|GetWorldDeltaSeconds) 2e+01) false false)
      (return false))))

(fn MoveGrappledPlayer
  (bind _returnvalue (Game|Player|GetPlayerPawn 0))
  (bind _asrope_decoy (Utilities|Casting|CastToRopeDecoy _returnvalue))
  (Character|LaunchCharacter _asrope_decoy (* (- (Variables|Default|GetHookLocation) (Transformation|GetActorLocation _returnvalue)) (* (Utilities|Time|GetWorldDeltaSeconds) 1.5e+02)) true true))