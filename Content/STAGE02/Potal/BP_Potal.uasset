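; BP_Potal is a portal actor that moves the player to the BeatNight_Stage_02 level.
; When BP_Player overlaps its Capsule and has CanGoStage2 set, it saves through BP_BeatNightGameModeBase and then opens that level.
; The construction script triggers a capture on its SceneCaptureComponentCube, so the cube capture is taken at construction.
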(event OnComponentBeginOverlap(Capsule)
  (params (OverlappedComponent :type Primitive%20Component%20Object%20Reference) (OtherActor :type Actor%20Object%20Reference) (OtherComp :type Primitive%20Component%20Object%20Reference) (OtherBodyIndex :type Integer) (bFromSweep :type Boolean) (SweepResult :type Hit%20Result%20Structure%20%28by%20ref%29))
  (bind _asbp_player (Utilities|Casting|CastToBP_Player OtherActor))
  (Utilities|IsValid _asbp_player
    (:Is%20Valid
      (if (Variables|/Script/UE4_BeatNight.BeatNightPlayer|GetbCanGoStage2 _asbp_player)
        (Class|BeatNightGameModeBase|SaveGame (.AsBP%20Beat%20Night%20Game%20Mode%20Base (Utilities|Casting|CastToBP_BeatNightGameModeBase (Game|GetGameMode))))
        (Game|OpenLevel(byObjectReference) "/Game/Maps/BeatNight_Stage_02.BeatNight_Stage_02")))))

(event EventBeginPlay)

(event Collision|EventActorBeginOverlap
  (params (OtherActor :type Actor%20Object%20Reference)))

(event EventTick
  (params (DeltaSeconds :type Float%20%28single-precision%29)))

(fn ConstructionScript
  (Rendering|SceneCapture|CaptureScene (Variables|Default|GetSceneCaptureComponentCube) :!class /Script/Engine.SceneCaptureComponentCube))