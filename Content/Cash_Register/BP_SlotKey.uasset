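; BP_SlotKey is a grabbable key actor in the cash register content, set to a fixed rotation on BeginPlay.
; Pickup disables mesh physics, attaches the root to the given component, records the Grabbed result, snaps the mesh to a hard-coded relative offset and rotation, and hides the particle effect.
; Drop re-enables physics, detaches the actor in world space and shows the particles again.
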(event EventBeginPlay
  (Transformation|SetActorRotation "50.000000, 0,90.000000"))

(event Collision|EventActorBeginOverlap
  (params (OtherActor :type Actor%20Object%20Reference)))

(event EventTick
  (params (DeltaSeconds :type Float%20%28single-precision%29)))

(event EventPickup
  (params (AttachTo :type Scene%20Component%20Object%20Reference))
  (Physics|SetSimulatePhysics (Variables|Default|GetStaticMesh) false)
  (bind _returnvalue (Transformation|AttachComponentToComponent (VehicleSound|GetRootComponent) AttachTo "None" "KeepWorld" "KeepWorld" "KeepWorld" false))
  (Variables|Default|SetGrabbed _returnvalue)
  ;[1 1 1] 추가사항(1/ )_손에 값 조정필요
  (Transformation|SetRelativeLocationAndRotation (Variables|Default|GetStaticMesh) "-10.000000,0.000000,-10.000000" "-180.000000,0.000000,90.000000" false false)
  (Rendering|SetVisibility (Variables|Default|GetParticleSystem) false false))

(event EventDrop
  (Physics|SetSimulatePhysics (Variables|Default|GetStaticMesh) true)
  (Transformation|DetachFromActor "KeepWorld" "KeepWorld" "KeepWorld")
  (Rendering|SetVisibility (Variables|Default|GetParticleSystem) true false))

(fn ConstructionScript)